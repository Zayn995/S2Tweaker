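; Ticking controller that adjusts the duration of S.T.A.L.K.E.R. 2 player movement sounds by gait.
; It parses a validated key=value save profile and runs only when audio.movement is 1.
; It inserts a Wwise effect on step, backpack and clothes mixer nodes, removing it without a valid player.
; Each tick, walk, run or limp factors and animation play rate set an inverse, clamped duration RTPC on the player's Ak components.
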(event `self.OnInitialized`
  (bind _loadedprofile (`self.LoadedProfile`))
  (bind _profilelines (`self.ProfileLines`))
  (bind _returnvalue (`KismetArrayLibrary.Array_Length` _profilelines))
  (bind _profiledata (`/S2TRuntimeLab/BP_S2TProfile.ProfileData` _loadedprofile))
  (bind _returnvalue_2 (`KismetStringLibrary.Len` _profiledata))
  (set `self.LoadedProfile` null)
  (bind _returnvalue_3 (`GameplayStatics.LoadGameFromSlot` (`self.ProfileSlot`)))
  (bind _asbp_s2tprofile (cast `/S2TRuntimeLab/BP_S2TProfile` _returnvalue_3)
    (:`then`
      (set `self.LoadedProfile` _asbp_s2tprofile))
    (:`CastFailed`
      _))
  (set `self.ProfileReady` false :!label _label)
  (`BlueprintMapLibrary.Map_Clear` (`self.ProfileValues`))
  (if (`KismetSystemLibrary.IsValid` _loadedprofile)
    (if (and (and (== (`/S2TRuntimeLab/BP_S2TProfile.ProfileSchema` _loadedprofile) 1) (>= _returnvalue_2 4)) (<= _returnvalue_2 64000))
      (set `self.ProfileLines` (`KismetStringLibrary.ParseIntoArray` _profiledata "\n" false))
      (if (and (>= _returnvalue 1) (<= _returnvalue 2048))
        (set `self.ProfileReady` true)
        (for (_array_element _array_index) _profilelines
          (if (== _array_index 0)
            (if (not (`KismetStringLibrary.EqualEqual_StrStr` _array_element "S2T1"))
              (set `self.ProfileReady` false :!label _label_2))
            (else
              (bind (_lefts _rights _returnvalue_4) (`KismetStringLibrary.Split` _array_element "="))
              (if _returnvalue_4
                (bind _returnvalue_5 (`KismetStringLibrary.Conv_StringToDouble` _rights))
                (if (and (and (and (and (`KismetStringLibrary.IsNumeric` _rights) (> _returnvalue_5 0.0)) (<= _returnvalue_5 100.0)) (> (`KismetStringLibrary.Len` _lefts) 0)) (not (`BlueprintMapLibrary.Map_Contains` (`self.ProfileValues`) _lefts)))
                  (`BlueprintMapLibrary.Map_Add` (`self.ProfileValues`) _lefts _returnvalue_5)
                  (else
                    (goto _label_2)))
                (else
                  (goto _label_2))))))
        (if (not (`self.ProfileReady`))
          (`BlueprintMapLibrary.Map_Clear` (`self.ProfileValues`)))))))

(event `ReleaseMovementSounds`
  (if (`self.StepApplied`)
    (`AkGameplayStatics.SetActorMixerEffect` (`KismetArrayLibrary.Array_Get` (`self.RootNodeIds`)) 3 (`self.EmptyEffect`)))
  (set `self.StepApplied` false)
  (if (`self.BackpackApplied`)
    (`AkGameplayStatics.SetActorMixerEffect` (`KismetArrayLibrary.Array_Get` (`self.RootNodeIds`) 1) 3 (`self.EmptyEffect`)))
  (set `self.BackpackApplied` false)
  (if (`self.ClothesApplied`)
    (`AkGameplayStatics.SetActorMixerEffect` (`KismetArrayLibrary.Array_Get` (`self.RootNodeIds`) 2) 3 (`self.EmptyEffect`)))
  (set `self.ClothesApplied` false)
  (set `self.CurrentNodeId` 0))

(event `self.OnWorldBeginPlay`
  (params (World :type "World Object Reference"))
  (bind (_value _returnvalue) (`BlueprintMapLibrary.Map_Find` (`self.ProfileValues`) "audio.movement"))
  (if (and (and (`self.ProfileReady`) _returnvalue) (== _value 1.0))
    (bind _returnvalue_2 (`|GenericCreateObject` self "/Script/AkAudio.AkEffectShareSet"))
    (set `self.EmptyEffect` _returnvalue_2)
    (`AkGameplayStatics.SetRTPCValue` (`self.DurationParameter`) 100.0)
    (set `self.AudioEnabled` true)
    (`self.SetTickEnabled` self true)))

(event `self.OnTick`
  (params (DeltaTime :type "Float (single-precision)"))
  (bind (_value _returnvalue) (`BlueprintMapLibrary.Map_Find` (`self.ProfileValues`) "audio.limp.run"))
  (bind (_value_2 _returnvalue_2) (`BlueprintMapLibrary.Map_Find` (`self.ProfileValues`) "audio.limp.walk"))
  (bind (_value_3 _returnvalue_3) (`BlueprintMapLibrary.Map_Find` (`self.ProfileValues`) "audio.run"))
  (bind (_value_4 _returnvalue_4) (`BlueprintMapLibrary.Map_Find` (`self.ProfileValues`) "audio.walk"))
  (if (`self.AudioEnabled`)
    (bind _aspc (cast `PC` (`GameplayStatics.GetPlayerPawn` 0))
      (:`then`
        (if (== (`self.CurrentNodeId`) 0)
          (bind _returnvalue_5 (`KismetSystemLibrary.LoadAsset_Blocking` (`KismetSystemLibrary.Conv_SoftObjPathToSoftObjRef` (`KismetSystemLibrary.MakeSoftObjectPath` "/Game/_STALKER2/Audio/WwiseAudio/Events/Human/Movement/SFX_Human_Step.SFX_Human_Step"))))
          (bind _asak_audio_event (cast `AkAudioEvent` _returnvalue_5))
          (set `self.MovementStepAnchor` _asak_audio_event)
          (`AkAudioType.LoadData` (`self.MovementStepAnchor`))
          (bind _returnvalue_6 (`KismetSystemLibrary.LoadAsset_Blocking` (`KismetSystemLibrary.Conv_SoftObjPathToSoftObjRef` (`KismetSystemLibrary.MakeSoftObjectPath` "/Game/_STALKER2/Audio/WwiseAudio/Events/Motion_Audio_Enveloper/SFX_MAE_PlayerClothes_Play.SFX_MAE_PlayerClothes_Play"))))
          (bind _asak_audio_event_2 (cast `AkAudioEvent` _returnvalue_6))
          (set `self.MovementClothesAnchor` _asak_audio_event_2)
          (`AkAudioType.LoadData` (`self.MovementClothesAnchor`))
          (bind _returnvalue_7 (`AkGameplayStatics.SetActorMixerEffect` (`KismetArrayLibrary.Array_Get` (`self.RootNodeIds`)) 3 (`self.Effect`)))
          (set `self.StepApplied` _returnvalue_7)
          (bind _returnvalue_8 (`AkGameplayStatics.SetActorMixerEffect` (`KismetArrayLibrary.Array_Get` (`self.RootNodeIds`) 1) 3 (`self.Effect`)))
          (set `self.BackpackApplied` _returnvalue_8)
          (bind _returnvalue_9 (`AkGameplayStatics.SetActorMixerEffect` (`KismetArrayLibrary.Array_Get` (`self.RootNodeIds`) 2) 3 (`self.Effect`)))
          (set `self.ClothesApplied` _returnvalue_9)
          (set `self.CurrentNodeId` 1))
        (bind _returnvalue_10 (`AnimationUtilitiesBPFunctionLibrary.GetCharacterAnimInstance` _aspc))
        (bind _asanim_instance_player (cast `AnimInstancePlayer` _returnvalue_10)
          (:`then`
            (set `self.ActiveSoundFactor` 1.0)
            (if (`PC.IsInCinematic` _aspc)
              (bind (_forwardvalue _rightvalue _playrate) (break `MovementPlayRateStructure` (`.MovementPlayRate` (break `AnimLocomotionData` (`AnimInstancePlayer.LocomotionData` _asanim_instance_player)))))
              (set `self.DurationPercent` (`KismetMathLibrary.FClamp` (/ 100.0 (* (`self.ActiveSoundFactor`) (`KismetMathLibrary.SelectFloat` _playrate 1.0 (and (and (`KismetSystemLibrary.IsValid` _asanim_instance_player) (> _playrate 0.0)) (not (`PC.IsInCinematic` _aspc)))))) 25.0 1600.0) :!label _label_3)
              (`AkGameplayStatics.SetRTPCValue` (`self.DurationParameter`) (`self.DurationPercent`) 0 _aspc)
              (for _array_element (`Actor.K2_GetComponentsByClass` _aspc "/Script/AkAudio.AkComponent")
                (bind _asakcomponent (cast `AkComponent` _array_element))
                (`AkComponent.SetRTPCValue` _asakcomponent (`self.DurationParameter`) (`self.DurationPercent`) 0 "S2T_MovementDuration"))
              (elif (and (`PC.IsLimping` _aspc) (not (`PC.IsCrouching` _aspc)))
                (if (`PC.IsWalking` _aspc)
                  (if (and _returnvalue_2 (> _value_2 0.0))
                    (set `self.ActiveSoundFactor` _value_2)
                    (goto _label_3)
                    (else
                      (goto _label_3)))
                  (elif (not (`PC.IsWalking` _aspc))
                    (if (and _returnvalue (> _value 0.0))
                      (set `self.ActiveSoundFactor` _value)
                      (goto _label_3)
                      (else
                        (goto _label_3)))))
                (elif (or (`PC.IsWalking` _aspc) (`PC.IsCrouching` _aspc))
                  (if (and _returnvalue_4 (> _value_4 0.0))
                    (set `self.ActiveSoundFactor` _value_4)
                    (goto _label_3)
                    (else
                      (goto _label_3)))
                  (elif (or (`PC.IsRunning` _aspc) (`PC.IsSprinting` _aspc))
                    (if (and _returnvalue_3 (> _value_3 0.0))
                      (set `self.ActiveSoundFactor` _value_3)
                      (goto _label_3)
                      (else
                        (goto _label_3)))
                    (else
                      (goto _label_3)))))))
          (:`CastFailed`
            (`self.ReleaseMovementSounds` :!label _label_4))))
      (:`CastFailed`
        (goto _label_4)))
    (else
      (goto _label_4))))

(event `ParseLoadedProfile`
  (goto _label))