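; World-subsystem-style Wwise controller that adjusts the player's weapon sound duration by per-action factors from the saved S2T profile.
; It validates the profile's key=value data, then each tick follows the live menu toggle and held weapon mesh.
; Profiled meshes get a mixer effect on their root and rattle audio nodes, plus a duration RTPC derived from jam, reload or equip montage factors.
; Effects and RTPC reset on release.
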(event `self.OnInitialized`
  (bind _loadedprofile (`self.LoadedProfile`))
  (bind _profilelines (`self.ProfileLines`))
  (bind _returnvalue (`KismetArrayLibrary.Array_Length` _profilelines))
  (bind _profiledata (`/S2TRuntimeLab/BP_S2TProfile.ProfileData` _loadedprofile))
  (bind _returnvalue_2 (`KismetStringLibrary.Len` _profiledata))
  (set `self.LoadedProfile` null)
  (bind _returnvalue_3 (`GameplayStatics.LoadGameFromSlot` (`self.ProfileSlot`)))
  (bind _asbp_s2tprofile (cast `/S2TRuntimeLab/BP_S2TProfile` _returnvalue_3)
    (:`then`
      (set `self.LoadedProfile` _asbp_s2tprofile))
    (:`CastFailed`
      _))
  (set `self.ProfileReady` false :!label _label)
  (`BlueprintMapLibrary.Map_Clear` (`self.ProfileValues`))
  (if (`KismetSystemLibrary.IsValid` _loadedprofile)
    (if (and (and (== (`/S2TRuntimeLab/BP_S2TProfile.ProfileSchema` _loadedprofile) 1) (>= _returnvalue_2 4)) (<= _returnvalue_2 64000))
      (set `self.ProfileLines` (`KismetStringLibrary.ParseIntoArray` _profiledata "\n"))
      (if (and (>= _returnvalue 1) (<= _returnvalue 2048))
        (set `self.ProfileReady` true)
        (for (_array_element _array_index) _profilelines
          (if (== _array_index 0)
            (if (not (`KismetStringLibrary.EqualEqual_StrStr` _array_element "S2T1"))
              (set `self.ProfileReady` false :!label _label_2))
            (else
              (bind (_lefts _rights _returnvalue_4) (`KismetStringLibrary.Split` _array_element "="))
              (if _returnvalue_4
                (bind _returnvalue_5 (`KismetStringLibrary.Conv_StringToDouble` _rights))
                (if (and (and (and (and (`KismetStringLibrary.IsNumeric` _rights) (> _returnvalue_5 0.0)) (<= _returnvalue_5 100.0)) (> (`KismetStringLibrary.Len` _lefts) 0)) (not (`BlueprintMapLibrary.Map_Contains` (`self.ProfileValues`) _lefts)))
                  (`BlueprintMapLibrary.Map_Add` (`self.ProfileValues`) _lefts _returnvalue_5)
                  (else
                    (goto _label_2)))
                (else
                  (goto _label_2))))))
        (if (not (`self.ProfileReady`))
          (`BlueprintMapLibrary.Map_Clear` (`self.ProfileValues`)))))))

(event `ReleaseRattles`
  (for _array_element (`self.OwnedRattleIds`)
    (`AkGameplayStatics.SetActorMixerEffect` _array_element 3 (`self.EmptyEffect`)))
  (`KismetArrayLibrary.Array_Clear` (`self.OwnedRattleIds`))
  (`KismetArrayLibrary.Array_Clear` (`self.RattleEvents`)))

(event `EnsureRattles`
  (for (_array_element _array_index) (`self.RattleEventPaths`)
    (bind _returnvalue (`KismetSystemLibrary.LoadAsset_Blocking` (`KismetSystemLibrary.Conv_SoftObjPathToSoftObjRef` (`KismetSystemLibrary.MakeSoftObjectPath` _array_element))))
    (bind _asak_audio_event (cast `AkAudioEvent` _returnvalue))
    (`KismetArrayLibrary.Array_AddUnique` (`self.RattleEvents`) _asak_audio_event)
    (`AkAudioType.LoadData` _asak_audio_event)
    (bind _item (`KismetArrayLibrary.Array_Get` (`self.RattleNodeIds`) _array_index))
    (bind _returnvalue_2 (`AkGameplayStatics.SetActorMixerEffect` _item 3 (`self.Effect`)))
    (if _returnvalue_2
      (`KismetArrayLibrary.Array_AddUnique` (`self.OwnedRattleIds`) _item))))

(event `ReleaseSoundNode`
  (if (`KismetSystemLibrary.IsValid` (`self.LastSoundPlayer`))
    (`AkGameplayStatics.SetRTPCValue` (`self.DurationParameter`) 100.0 0 (`self.LastSoundPlayer`))
    (for _array_element (`Actor.K2_GetComponentsByClass` (`self.LastSoundPlayer`) "/Script/AkAudio.AkComponent")
      (bind _asakcomponent (cast `AkComponent` _array_element))
      (`AkComponent.SetRTPCValue` _asakcomponent (`self.DurationParameter`) 100.0 0 "S2T_ActionDuration")))
  (set `self.LastSoundPlayer` null)
  (`self.ReleaseRattles`)
  (if (`self.NodeApplied`)
    (`AkGameplayStatics.SetActorMixerEffect` (`KismetArrayLibrary.Array_Get` (`self.RootNodeIds`) (- (`self.CurrentNodeId`) 1)) 3 (`self.EmptyEffect`))
    (set `self.NodeApplied` false)))

(event `self.OnWorldBeginPlay`
  (params (World :type "World Object Reference"))
  (bind (_value _returnvalue) (`BlueprintMapLibrary.Map_Find` (`self.ProfileValues`) "menu.enabled"))
  (bind (_value_2 _returnvalue_2) (`BlueprintMapLibrary.Map_Find` (`self.ProfileValues`) "audio.enabled"))
  (if (or (and (and (`self.ProfileReady`) _returnvalue_2) (== _value_2 1.0)) (and (and (`self.ProfileReady`) _returnvalue) (== _value 1.0)))
    (bind _returnvalue_3 (`|GenericCreateObject` self "/Script/AkAudio.AkEffectShareSet"))
    (set `self.EmptyEffect` _returnvalue_3)
    (`AkGameplayStatics.SetRTPCValue` (`self.DurationParameter`) 100.0)
    (set `self.AudioEnabled` true)
    (`self.SetTickEnabled` self true)))

(event `self.OnTick`
  (params (DeltaTime :type "Float (single-precision)"))
  (bind _returnvalue (`GameplayStatics.GetPlayerController` 0))
  (bind (_value _returnvalue_2) (`BlueprintMapLibrary.Map_Find` (`self.ProfileValues`) "audio.jam"))
  (bind (_value_2 _returnvalue_3) (`BlueprintMapLibrary.Map_Find` (`self.ProfileValues`) "audio.reload"))
  (bind (_value_3 _returnvalue_4) (`BlueprintMapLibrary.Map_Find` (`self.ProfileValues`) "menu.sound.weapon"))
  (bind (_value_4 _returnvalue_5) (`BlueprintMapLibrary.Map_Find` (`self.ProfileValues`) "menu.enabled"))
  (set `self.MenuSoundRequested` (`self.AudioEnabled`))
  (if (and (and (`self.ProfileReady`) _returnvalue_5) (== _value_4 1.0))
    (set `self.MenuSoundRequested` (and _returnvalue_4 (== _value_3 2.0)))
    (if (`KismetSystemLibrary.IsValid` (`self.LiveMenu`))
      (if (and (`KismetSystemLibrary.IsValid` _returnvalue) (`KismetSystemLibrary.IsValid` (`self.LoadedProfile`))) :!label _label_3
        (if (and (and (and (and (`Controller.IsLocalController` _returnvalue) (== (`UserWidget.GetOwningPlayer` (`self.LiveMenu`)) _returnvalue)) (`Widget.IsInViewport` (`self.LiveMenu`))) (`/S2TRuntimeLab/Menu/WBP_S2TMenu.ProfileReady` (`self.LiveMenu`))) (`KismetStringLibrary.EqualEqual_StrStr` (`/S2TRuntimeLab/Menu/WBP_S2TMenu.SourceProfile` (`self.LiveMenu`)) (`/S2TRuntimeLab/BP_S2TProfile.ProfileData` (`self.LoadedProfile`))))
          (set `self.MenuSoundRequested` (`/S2TRuntimeLab/Menu/WBP_S2TMenu.WeaponSound` (`self.LiveMenu`)))
          (else
            (set `self.LiveMenu` null :!label _label_4)))
        (else
          (goto _label_4)))
      (else
        (set `self.MenuSearchElapsed` (+ (`self.MenuSearchElapsed`) DeltaTime))
        (if (>= (`self.MenuSearchElapsed`) 0.5)
          (set `self.MenuSearchElapsed` 0.0)
          (bind _foundwidgets (`WidgetBlueprintLibrary.GetAllWidgetsOfClass` "/S2TRuntimeLab/Menu/WBP_S2TMenu.WBP_S2TMenu_C"))
          (if (== (`KismetArrayLibrary.Array_Length` _foundwidgets) 1)
            (bind _aswbp_s2tmenu (cast `/S2TRuntimeLab/Menu/WBP_S2TMenu` (`KismetArrayLibrary.Array_Get` _foundwidgets))
              (:`then`
                (set `self.LiveMenu` _aswbp_s2tmenu)
                (goto _label_3))
              (:`CastFailed`
                _)))))))
  (if (and (`self.AudioEnabled`) (`self.MenuSoundRequested`))
    (bind _aspc (cast `PC` (`GameplayStatics.GetPlayerPawn` 0))
      (:`then`
        (bind _returnvalue_6 (`PC.GetWeaponInHandsMeshComponent` _aspc))
        (if (`KismetSystemLibrary.IsValid` _returnvalue_6)
          (bind _returnvalue_7 (`SkeletalMeshComponent.GetSkeletalMeshAsset` _returnvalue_6))
          (bind _returnvalue_8 (`KismetSystemLibrary.GetObjectName` _returnvalue_7))
          (bind (_value_5 _returnvalue_9) (`BlueprintMapLibrary.Map_Find` (`self.ProfileValues`) (`KismetStringLibrary.Concat_StrStr` "audio.mesh." _returnvalue_8)))
          (bind _returnvalue_10 (`KismetMathLibrary.FTrunc` _value_5))
          (if (and (and (and (`KismetSystemLibrary.IsValid` _returnvalue_7) _returnvalue_9) (>= _returnvalue_10 1)) (<= _returnvalue_10 (`KismetArrayLibrary.Array_Length` (`self.RootNodeIds`))))
            (if (`KismetStringLibrary.NotEqual_StrStr` _returnvalue_8 (`self.CurrentMesh`))
              (`self.ReleaseSoundNode`)
              (set `self.CurrentMesh` _returnvalue_8)
              (set `self.CurrentNodeId` _returnvalue_10)
              (bind _returnvalue_11 (`KismetSystemLibrary.LoadAsset_Blocking` (`KismetSystemLibrary.Conv_SoftObjPathToSoftObjRef` (`KismetSystemLibrary.MakeSoftObjectPath` (`KismetArrayLibrary.Array_Get` (`self.RootEventPaths`) (- _returnvalue_10 1))))))
              (bind _asak_audio_event (cast `AkAudioEvent` _returnvalue_11))
              (set `self.LoadedEvent` _asak_audio_event)
              (`AkAudioType.LoadData` (`self.LoadedEvent`))
              (bind _returnvalue_12 (`AkGameplayStatics.SetActorMixerEffect` (`KismetArrayLibrary.Array_Get` (`self.RootNodeIds`) (- (`self.CurrentNodeId`) 1)) 3 (`self.Effect`)))
              (set `self.NodeApplied` _returnvalue_12)
              (`self.EnsureRattles`))
            (set `self.ActiveSoundFactor` 1.0)
            (bind _returnvalue_13 (`SkeletalMeshComponent.GetAnimInstance` _returnvalue_6))
            (if (`KismetSystemLibrary.IsValid` _returnvalue_13)
              (bind _returnvalue_14 (`AnimInstance.GetCurrentActiveMontage` _returnvalue_13))
              (bind _returnvalue_15 (`KismetSystemLibrary.GetObjectName` _returnvalue_14))
              (if (and (`KismetSystemLibrary.IsValid` _returnvalue_14) (`KismetStringLibrary.Contains` _returnvalue_15 "jam"))
                (if (and _returnvalue_2 (> _value 0.0))
                  (set `self.ActiveSoundFactor` _value))
                (elif (and (`KismetSystemLibrary.IsValid` _returnvalue_14) (`KismetStringLibrary.Contains` _returnvalue_15 "reload"))
                  (if (and _returnvalue_3 (> _value_2 0.0))
                    (set `self.ActiveSoundFactor` _value_2))
                  (elif (and (`KismetSystemLibrary.IsValid` _returnvalue_14) (`KismetStringLibrary.Contains` _returnvalue_15 "equip"))
                    (bind (_value_6 _returnvalue_16) (`BlueprintMapLibrary.Map_Find` (`self.ProfileValues`) (`KismetStringLibrary.Concat_StrStr` "audio.equip." _returnvalue_8)))
                    (if (and _returnvalue_16 (> _value_6 0.0))
                      (set `self.ActiveSoundFactor` _value_6))))))
            (set `self.DurationPercent` 100.0)
            (set `self.DurationPercent` (`KismetMathLibrary.FClamp` (/ 100.0 (`self.ActiveSoundFactor`)) 25.0 1600.0))
            (`AkGameplayStatics.SetRTPCValue` (`self.DurationParameter`) (`self.DurationPercent`) 0 _aspc)
            (set `self.LastSoundPlayer` _aspc)
            (for _array_element (`Actor.K2_GetComponentsByClass` _aspc "/Script/AkAudio.AkComponent")
              (bind _asakcomponent (cast `AkComponent` _array_element))
              (`AkComponent.SetRTPCValue` _asakcomponent (`self.DurationParameter`) (`self.DurationPercent`) 0 "S2T_ActionDuration"))
            (else
              (`self.ReleaseSoundNode` :!label _label_5)
              (set `self.CurrentMesh` "")))
          (else
            (goto _label_5))))
      (:`CastFailed`
        (goto _label_5)))
    (else
      (goto _label_5))))

(event `self.PreDeinitialize`
  (`self.SetTickEnabled` self false)
  (set `self.LiveMenu` null)
  (`self.ReleaseSoundNode`))

(event `ParseLoadedProfile`
  (goto _label))