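; World-lifecycle controller that provides the S2T menu on F10 when a saved profile enables it.
; It loads the profile and strictly parses its versioned key=value data into a map, discarding everything on any bad entry.
; Tick creates a hidden widget for the local player, opening it only during unblocked gameplay when its profile matches the loaded one.
; Losing the valid player or controller, or deinitializing, tears the widget down.
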(event `self.OnInitialized`
  (bind _loadedprofile (`self.LoadedProfile`))
  (bind _profilelines (`self.ProfileLines`))
  (bind _returnvalue (`KismetArrayLibrary.Array_Length` _profilelines))
  (bind _profiledata (`/S2TRuntimeLab/BP_S2TProfile.ProfileData` _loadedprofile))
  (bind _returnvalue_2 (`KismetStringLibrary.Len` _profiledata))
  (set `self.LoadedProfile` null)
  (bind _returnvalue_3 (`GameplayStatics.LoadGameFromSlot` (`self.ProfileSlot`)))
  (bind _asbp_s2tprofile (cast `/S2TRuntimeLab/BP_S2TProfile` _returnvalue_3)
    (:`then`
      (set `self.LoadedProfile` _asbp_s2tprofile))
    (:`CastFailed`
      _))
  (set `self.ProfileReady` false :!label _label)
  (`BlueprintMapLibrary.Map_Clear` (`self.ProfileValues`))
  (if (`KismetSystemLibrary.IsValid` _loadedprofile)
    (if (and (and (== (`/S2TRuntimeLab/BP_S2TProfile.ProfileSchema` _loadedprofile) 1) (>= _returnvalue_2 4)) (<= _returnvalue_2 64000))
      (set `self.ProfileLines` (`KismetStringLibrary.ParseIntoArray` _profiledata "\n"))
      (if (and (>= _returnvalue 1) (<= _returnvalue 2048))
        (set `self.ProfileReady` true)
        (for (_array_element _array_index) _profilelines
          (if (== _array_index 0)
            (if (not (`KismetStringLibrary.EqualEqual_StrStr` _array_element "S2T1"))
              (set `self.ProfileReady` false :!label _label_2))
            (else
              (bind (_lefts _rights _returnvalue_4) (`KismetStringLibrary.Split` _array_element "="))
              (if _returnvalue_4
                (bind _returnvalue_5 (`KismetStringLibrary.Conv_StringToDouble` _rights))
                (if (and (and (and (and (`KismetStringLibrary.IsNumeric` _rights) (> _returnvalue_5 0.0)) (<= _returnvalue_5 100.0)) (> (`KismetStringLibrary.Len` _lefts) 0)) (not (`BlueprintMapLibrary.Map_Contains` (`self.ProfileValues`) _lefts)))
                  (`BlueprintMapLibrary.Map_Add` (`self.ProfileValues`) _lefts _returnvalue_5)
                  (else
                    (goto _label_2)))
                (else
                  (goto _label_2))))))
        (if (not (`self.ProfileReady`))
          (`BlueprintMapLibrary.Map_Clear` (`self.ProfileValues`)))))))

(event `self.OnWorldBeginPlay`
  (params (World :type "World Object Reference"))
  (bind (_value _returnvalue) (`BlueprintMapLibrary.Map_Find` (`self.ProfileValues`) "menu.enabled"))
  (if (and (and (`self.ProfileReady`) _returnvalue) (== _value 1.0))
    (set `self.MenuEnabled` true)
    (`self.SetTickEnabled` self true)))

(event `self.PreDeinitialize`
  (set `self.MenuEnabled` false)
  (`self.SetTickEnabled` self false)
  (if (`KismetSystemLibrary.IsValid` (`self.Menu`)) :!label _label_3
    (if (`/S2TRuntimeLab/Menu/WBP_S2TMenu.MenuOpen` (`self.Menu`))
      (if (`KismetSystemLibrary.IsValid` (`self.OwnerController`))
        (if (and (or (`Widget.HasAnyUserFocus` (`self.Menu`)) (`Widget.HasFocusedDescendants` (`self.Menu`))) (== (`self.OwnerController`) (`UserWidget.GetOwningPlayer` (`self.Menu`))))
          (`/S2TRuntimeLab/Menu/WBP_S2TMenu.CloseMenu` (`self.Menu`)))))
    (set `/S2TRuntimeLab/Menu/WBP_S2TMenu.MenuOpen` false (`self.Menu`))
    (`Widget.RemoveFromParent` (`self.Menu`)))
  (set `self.Menu` null)
  (set `self.OwnerController` null))

(event `self.OnTick`
  (params (DeltaTime :type "Float (single-precision)"))
  (bind _returnvalue (`GameplayStatics.GetPlayerController` 0))
  (if (`self.MenuEnabled`)
    (if (`KismetSystemLibrary.IsValid` _returnvalue)
      (if (`Controller.IsLocalController` _returnvalue)
        (bind _aspc (cast `PC` (`GameplayStatics.GetPlayerPawn` 0))
          (:`then`
            (if (and (`Obj.IsCurrentPlayer` _aspc) (`Pawn.IsPlayerControlled` _aspc))
              (if (`KismetSystemLibrary.IsValid` (`self.Menu`))
                (if (== _returnvalue (`self.OwnerController`))
                  (if (not (`/S2TRuntimeLab/Menu/WBP_S2TMenu.MenuOpen` (`self.Menu`)))
                    (if (`/S2TRuntimeLab/Menu/WBP_S2TMenu.ProfileReady` (`self.Menu`))
                      (if (`KismetStringLibrary.EqualEqual_StrStr` (`/S2TRuntimeLab/Menu/WBP_S2TMenu.SourceProfile` (`self.Menu`)) (`/S2TRuntimeLab/BP_S2TProfile.ProfileData` (`self.LoadedProfile`)))
                        (if (and (and (and (and (not (`GameplayStatics.IsGamePaused`)) (not (`PlayerController.bShowMouseCursor` _returnvalue))) (not (`Controller.IsMoveInputIgnored` _returnvalue))) (not (`Controller.IsLookInputIgnored` _returnvalue))) (not (`Obj.IsInCinematic` _aspc)))
                          (if (`PlayerController.WasInputKeyJustPressed` _returnvalue "F10")
                            (`/S2TRuntimeLab/Menu/WBP_S2TMenu.OpenMenu` (`self.Menu`)))))))
                  (else
                    (goto _label_3)))
                (else
                  (bind _returnvalue_2 (`|CreateWidget` "/S2TRuntimeLab/Menu/WBP_S2TMenu.WBP_S2TMenu_C" _returnvalue))
                  (set `self.Menu` _returnvalue_2)
                  (if (`KismetSystemLibrary.IsValid` (`self.Menu`))
                    (set `self.OwnerController` _returnvalue)
                    (set `/S2TRuntimeLab/Menu/WBP_S2TMenu.ProfileSlot` (`self.ProfileSlot`) (`self.Menu`))
                    (`Widget.SetVisibility` (`self.Menu`) "Hidden")
                    (`UserWidget.AddToViewport` (`self.Menu`) 100))))
              (else
                (goto _label_3))))
          (:`CastFailed`
            (goto _label_3)))
        (else
          (goto _label_3)))
      (else
        (goto _label_3)))))

(event `ParseLoadedProfile`
  (goto _label))