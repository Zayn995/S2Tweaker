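; Runtime controller that changes player animation speed per gait using multipliers from a saved S2T profile.
; On initialization it validates and parses the profile into a key-to-multiplier map, enabling tick at BeginPlay if movement keys exist.
; Each tick it scales body and shadow mesh GlobalAnimRateScale by gait, counter-scaling their active montages to preserve playback speed.
; Cached original rates are restored during cinematics, only overwriting montage rates it last wrote.
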(event `self.OnInitialized`
  (bind _loadedprofile (`self.LoadedProfile`))
  (bind _profilelines (`self.ProfileLines`))
  (bind _returnvalue (`KismetArrayLibrary.Array_Length` _profilelines))
  (bind _profiledata (`/S2TRuntimeLab/BP_S2TProfile.ProfileData` _loadedprofile))
  (bind _returnvalue_2 (`KismetStringLibrary.Len` _profiledata))
  (set `self.LoadedProfile` null)
  (bind _returnvalue_3 (`GameplayStatics.LoadGameFromSlot` (`self.ProfileSlot`)))
  (bind _asbp_s2tprofile (cast `/S2TRuntimeLab/BP_S2TProfile` _returnvalue_3)
    (:`then`
      (set `self.LoadedProfile` _asbp_s2tprofile))
    (:`CastFailed`
      _))
  (set `self.ProfileReady` false :!label _label)
  (`BlueprintMapLibrary.Map_Clear` (`self.ProfileValues`))
  (if (`KismetSystemLibrary.IsValid` _loadedprofile)
    (if (and (and (== (`/S2TRuntimeLab/BP_S2TProfile.ProfileSchema` _loadedprofile) 1) (>= _returnvalue_2 4)) (<= _returnvalue_2 64000))
      (set `self.ProfileLines` (`KismetStringLibrary.ParseIntoArray` _profiledata "\n" false))
      (if (and (>= _returnvalue 1) (<= _returnvalue 2048))
        (set `self.ProfileReady` true)
        (for (_array_element _array_index) _profilelines
          (if (== _array_index 0)
            (if (not (`KismetStringLibrary.EqualEqual_StrStr` _array_element "S2T1"))
              (set `self.ProfileReady` false :!label _label_2))
            (else
              (bind (_lefts _rights _returnvalue_4) (`KismetStringLibrary.Split` _array_element "="))
              (if _returnvalue_4
                (bind _returnvalue_5 (`KismetStringLibrary.Conv_StringToDouble` _rights))
                (if (and (and (and (and (`KismetStringLibrary.IsNumeric` _rights) (> _returnvalue_5 0.0)) (<= _returnvalue_5 100.0)) (> (`KismetStringLibrary.Len` _lefts) 0)) (not (`BlueprintMapLibrary.Map_Contains` (`self.ProfileValues`) _lefts)))
                  (`BlueprintMapLibrary.Map_Add` (`self.ProfileValues`) _lefts _returnvalue_5)
                  (else
                    (goto _label_2)))
                (else
                  (goto _label_2))))))
        (if (not (`self.ProfileReady`))
          (`BlueprintMapLibrary.Map_Clear` (`self.ProfileValues`)))))))

(event `ParseLoadedProfile`
  (goto _label))

(event `self.OnTick`
  (params (DeltaTime :type "Float (single-precision)"))
  (if (`self.LabAutoGait`)
    (bind _aspc (cast `PC` (`GameplayStatics.GetPlayerPawn` 0))
      (:`then`
        (if (`PC.IsInCinematic` _aspc)
          (`self.ReleaseProfileComponentRates` :!label _label_3)
          (`self.ReleaseProfileReloadRates`)
          (else
            (if (`PC.IsCrouching` _aspc)
              (set `self.ActiveGaitKey` "movement.crouch")
              (elif (`PC.IsLimping` _aspc)
                (if (`PC.IsWalking` _aspc)
                  (set `self.ActiveGaitKey` "movement.limp.walk")
                  (else
                    (set `self.ActiveGaitKey` "movement.limp.run")))
                (elif (`PC.IsSprinting` _aspc)
                  (set `self.ActiveGaitKey` "movement.sprint")
                  (elif (`PC.IsWalking` _aspc)
                    (set `self.ActiveGaitKey` "movement.walk")
                    (elif (`PC.IsRunning` _aspc)
                      (set `self.ActiveGaitKey` "movement.run")
                      (else
                        (set `self.ActiveGaitKey` "unconfigured.native_default")))))))
            (for _array_element (`Actor.K2_GetComponentsByClass` _aspc "/Script/Engine.SkeletalMeshComponent")
              (bind _asskeletal_mesh_component (cast `SkeletalMeshComponent` _array_element))
              (bind _returnvalue (`KismetSystemLibrary.GetObjectName` _asskeletal_mesh_component))
              (if (or (`KismetStringLibrary.EqualEqual_StrStr` _returnvalue "CharacterMesh0") (`KismetStringLibrary.EqualEqual_StrStr` _returnvalue "ShadowMesh"))
                (`self.ApplyProfileComponentRate` _asskeletal_mesh_component (`self.ActiveGaitKey`))
                (set `self.GaitDispatchCount` (+ (`self.GaitDispatchCount`) 1))
                (`self.ApplyProfileReloadRate` _asskeletal_mesh_component :!label _label_4)
                (elif (`KismetStringLibrary.StartsWith` _returnvalue "WeaponInHandsMesh")
                  (goto _label_4)))))))
      (:`CastFailed`
        (goto _label_3)))
    (else
      (goto _label_3))))

(event `self.OnWorldBeginPlay`
  (params (World :type "World Object Reference"))
  (if (and (`self.ProfileReady`) (or (or (or (or (or (`BlueprintMapLibrary.Map_Contains` (`self.ProfileValues`) "movement.crouch") (`BlueprintMapLibrary.Map_Contains` (`self.ProfileValues`) "movement.sprint")) (`BlueprintMapLibrary.Map_Contains` (`self.ProfileValues`) "movement.limp.walk")) (`BlueprintMapLibrary.Map_Contains` (`self.ProfileValues`) "movement.limp.run")) (`BlueprintMapLibrary.Map_Contains` (`self.ProfileValues`) "movement.walk")) (`BlueprintMapLibrary.Map_Contains` (`self.ProfileValues`) "movement.run")))
    (set `self.LabAutoGait` true)
    (`self.SetTickEnabled` true)))

(event `ApplyProfileComponentRate`
  (params (TargetMesh :type "SkeletalMeshComponent Object Reference") (ProfileKey :type String))
  (bind _value (`BlueprintMapLibrary.Map_Find` (`self.OriginalComponentRates`) TargetMesh))
  (bind (_value_2 _returnvalue) (`BlueprintMapLibrary.Map_Find` (`self.ProfileValues`) ProfileKey))
  (if (`KismetSystemLibrary.IsValid` TargetMesh)
    (if (not (`.ReturnValue` (`BlueprintMapLibrary.Map_Find` (`self.OriginalComponentRates`) TargetMesh)))
      (`BlueprintMapLibrary.Map_Add` (`self.OriginalComponentRates`) TargetMesh (`SkeletalMeshComponent.GlobalAnimRateScale` TargetMesh)))
    (set `self.ComputedComponentRate` _value)
    (if (and (`self.ProfileReady`) _returnvalue)
      (set `self.ComputedComponentRate` (* _value _value_2)))
    (set `SkeletalMeshComponent.GlobalAnimRateScale` (`self.ComputedComponentRate`) TargetMesh)))

(event `ReleaseProfileComponentRates`
  (bind _keys (`BlueprintMapLibrary.Map_Keys` (`self.OriginalComponentRates`)))
  (for _array_element _keys
    (if (`KismetSystemLibrary.IsValid` _array_element)
      (set `SkeletalMeshComponent.GlobalAnimRateScale` (`BlueprintMapLibrary.Map_Find` (`self.OriginalComponentRates`) _array_element) _array_element)))
  (`BlueprintMapLibrary.Map_Clear` (`self.OriginalComponentRates`)))

(event `ApplyProfileReloadRate`
  (params (TargetMesh :type "SkeletalMeshComponent Object Reference"))
  (bind _returnvalue (`SkeletalMeshComponent.GetAnimInstance` TargetMesh))
  (bind _globalanimratescale (`SkeletalMeshComponent.GlobalAnimRateScale` TargetMesh))
  (bind (_value _returnvalue_2) (`BlueprintMapLibrary.Map_Find` (`self.LastWrittenMontageRates`) _returnvalue))
  (bind _value_2 (`BlueprintMapLibrary.Map_Find` (`self.OriginalMontageRates`) _returnvalue))
  (bind (_value_3 _returnvalue_3) (`BlueprintMapLibrary.Map_Find` (`self.TrackedProfileMontages`) _returnvalue))
  (bind _returnvalue_4 (`AnimInstance.GetCurrentActiveMontage` _returnvalue))
  (bind (_value_4 _returnvalue_5) (`BlueprintMapLibrary.Map_Find` (`self.OriginalComponentRates`) TargetMesh))
  (bind _returnvalue_6 (/ (* (`self.ComputedMontageRate`) _value_4) _globalanimratescale))
  (if (`KismetSystemLibrary.IsValid` TargetMesh)
    (if (`KismetSystemLibrary.IsValid` _returnvalue)
      (if (`KismetSystemLibrary.IsValid` _returnvalue_4)
        (if (not (and (and _returnvalue_3 (== _value_3 _returnvalue_4)) (and _returnvalue_2 (`KismetMathLibrary.NearlyEqual_FloatFloat` (`AnimInstance.Montage_GetPlayRate` _returnvalue _returnvalue_4) _value 1e-06))))
          (if (and (and (and (and _returnvalue_3 (`KismetSystemLibrary.IsValid` _value_3)) (`AnimInstance.Montage_IsActive` _returnvalue _value_3)) _returnvalue_2) (`KismetMathLibrary.NearlyEqual_FloatFloat` (`AnimInstance.Montage_GetPlayRate` _returnvalue _value_3) _value 1e-06))
            (`AnimInstance.Montage_SetPlayRate` _returnvalue _value_3 _value_2))
          (`BlueprintMapLibrary.Map_Add` (`self.OriginalMontageRates`) _returnvalue (`AnimInstance.Montage_GetPlayRate` _returnvalue _returnvalue_4))
          (`BlueprintMapLibrary.Map_Add` (`self.TrackedProfileMontages`) _returnvalue _returnvalue_4))
        (set `self.ComputedMontageRate` _value_2)
        (if (and _returnvalue_5 (> _globalanimratescale 0.0))
          (if (not (`KismetMathLibrary.NearlyEqual_FloatFloat` (`AnimInstance.Montage_GetPlayRate` _returnvalue _returnvalue_4) _returnvalue_6 1e-06))
            (`AnimInstance.Montage_SetPlayRate` _returnvalue _returnvalue_4 _returnvalue_6)
            (`BlueprintMapLibrary.Map_Add` (`self.LastWrittenMontageRates`) _returnvalue _returnvalue_6)
            (set `self.ReloadApplyCount` (+ (`self.ReloadApplyCount`) 1))))
        (else
          (if (and (and (and (and _returnvalue_3 (`KismetSystemLibrary.IsValid` _value_3)) (`AnimInstance.Montage_IsActive` _returnvalue _value_3)) _returnvalue_2) (`KismetMathLibrary.NearlyEqual_FloatFloat` (`AnimInstance.Montage_GetPlayRate` _returnvalue _value_3) _value 1e-06))
            (`AnimInstance.Montage_SetPlayRate` _returnvalue _value_3 _value_2))
          (`BlueprintMapLibrary.Map_Remove` (`self.OriginalMontageRates`) _returnvalue)
          (`BlueprintMapLibrary.Map_Remove` (`self.TrackedProfileMontages`) _returnvalue)
          (`BlueprintMapLibrary.Map_Remove` (`self.LastWrittenMontageRates`) _returnvalue))))))

(event `ReleaseProfileReloadRates`
  (bind _keys (`BlueprintMapLibrary.Map_Keys` (`self.TrackedProfileMontages`)))
  (for _array_element _keys
    (if (`KismetSystemLibrary.IsValid` _array_element)
      (bind (_value _returnvalue) (`BlueprintMapLibrary.Map_Find` (`self.TrackedProfileMontages`) _array_element))
      (bind (_value_2 _returnvalue_2) (`BlueprintMapLibrary.Map_Find` (`self.LastWrittenMontageRates`) _array_element))
      (if (and (and (and (and _returnvalue (`KismetSystemLibrary.IsValid` _value)) (`AnimInstance.Montage_IsActive` _array_element _value)) _returnvalue_2) (`KismetMathLibrary.NearlyEqual_FloatFloat` (`AnimInstance.Montage_GetPlayRate` _array_element _value) _value_2 1e-06))
        (`AnimInstance.Montage_SetPlayRate` _array_element _value (`BlueprintMapLibrary.Map_Find` (`self.OriginalMontageRates`) _array_element)))))
  (`BlueprintMapLibrary.Map_Clear` (`self.OriginalMontageRates`))
  (`BlueprintMapLibrary.Map_Clear` (`self.TrackedProfileMontages`))
  (`BlueprintMapLibrary.Map_Clear` (`self.LastWrittenMontageRates`)))