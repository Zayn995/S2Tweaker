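; Tickable world subsystem that scales idle sway amplitude on the player's anim instances from a saved S2T profile.
; It validates the profile's key=value data, then takes the sway factor from it or from a matching live WBP_S2TMenu.
; Original and last-written values are tracked per instance, preventing compounding and preserving external changes.
; Sway is released at factor 1, in cinematics, without a valid pawn, or on teardown.
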(event `self.OnInitialized`
  (bind _loadedprofile (`self.LoadedProfile`))
  (bind _profilelines (`self.ProfileLines`))
  (bind _returnvalue (`KismetArrayLibrary.Array_Length` _profilelines))
  (bind _profiledata (`/S2TRuntimeLab/BP_S2TProfile.ProfileData` _loadedprofile))
  (bind _returnvalue_2 (`KismetStringLibrary.Len` _profiledata))
  (set `self.LoadedProfile` null)
  (bind _returnvalue_3 (`GameplayStatics.LoadGameFromSlot` (`self.ProfileSlot`)))
  (bind _asbp_s2tprofile (cast `/S2TRuntimeLab/BP_S2TProfile` _returnvalue_3)
    (:`then`
      (set `self.LoadedProfile` _asbp_s2tprofile))
    (:`CastFailed`
      _))
  (set `self.ProfileReady` false :!label _label)
  (`BlueprintMapLibrary.Map_Clear` (`self.ProfileValues`))
  (if (`KismetSystemLibrary.IsValid` _loadedprofile)
    (if (and (and (== (`/S2TRuntimeLab/BP_S2TProfile.ProfileSchema` _loadedprofile) 1) (>= _returnvalue_2 4)) (<= _returnvalue_2 64000))
      (set `self.ProfileLines` (`KismetStringLibrary.ParseIntoArray` _profiledata "\n"))
      (if (and (>= _returnvalue 1) (<= _returnvalue 2048))
        (set `self.ProfileReady` true)
        (for (_array_element _array_index) _profilelines
          (if (== _array_index 0)
            (if (not (`KismetStringLibrary.EqualEqual_StrStr` _array_element "S2T1"))
              (set `self.ProfileReady` false :!label _label_2))
            (else
              (bind (_lefts _rights _returnvalue_4) (`KismetStringLibrary.Split` _array_element "="))
              (if _returnvalue_4
                (bind _returnvalue_5 (`KismetStringLibrary.Conv_StringToDouble` _rights))
                (if (and (and (and (and (`KismetStringLibrary.IsNumeric` _rights) (> _returnvalue_5 0.0)) (<= _returnvalue_5 100.0)) (> (`KismetStringLibrary.Len` _lefts) 0)) (not (`BlueprintMapLibrary.Map_Contains` (`self.ProfileValues`) _lefts)))
                  (`BlueprintMapLibrary.Map_Add` (`self.ProfileValues`) _lefts _returnvalue_5)
                  (else
                    (goto _label_2)))
                (else
                  (goto _label_2))))))
        (if (not (`self.ProfileReady`))
          (`BlueprintMapLibrary.Map_Clear` (`self.ProfileValues`)))))))

(event `ApplySway`
  (params (Target :type "AnimInstancePlayer Object Reference") (Factor :type "Float (double-precision)"))
  (bind (_basecurve _staminaamplitudecurve _staminacycletimecurve _initialdelay _standcycletimemodifier _standamplitudexmodifier _standamplitudeymodifier _crouchcycletimemodifier _crouchamplitudexmodifier _crouchamplitudeymodifier _movecycletimemodifier _moveamplitudexmodifier _moveamplitudeymodifier) (break `AnimPlayerIdleSwayData` (`self.WorkingSway`)))
  (bind (_basecurve_2 _staminaamplitudecurve_2 _staminacycletimecurve_2 _initialdelay_2 _standcycletimemodifier_2 _standamplitudexmodifier_2 _standamplitudeymodifier_2 _crouchcycletimemodifier_2 _crouchamplitudexmodifier_2 _crouchamplitudeymodifier_2 _movecycletimemodifier_2 _moveamplitudexmodifier_2 _moveamplitudeymodifier_2) (break `AnimPlayerIdleSwayData` (`self.BaselineSway`)))
  (bind (_value _returnvalue) (`BlueprintMapLibrary.Map_Find` (`self.LastSway`) Target))
  (bind (_value_2 _returnvalue_2) (`BlueprintMapLibrary.Map_Find` (`self.OriginalSway`) Target))
  (bind (_basecurve_3 _staminaamplitudecurve_3 _staminacycletimecurve_3 _initialdelay_3 _standcycletimemodifier_3 _standamplitudexmodifier_3 _standamplitudeymodifier_3 _crouchcycletimemodifier_3 _crouchamplitudexmodifier_3 _crouchamplitudeymodifier_3 _movecycletimemodifier_3 _moveamplitudexmodifier_3 _moveamplitudeymodifier_3) (break `AnimPlayerIdleSwayData` _value_2))
  (bind (_basecurve_4 _staminaamplitudecurve_4 _staminacycletimecurve_4 _initialdelay_4 _standcycletimemodifier_4 _standamplitudexmodifier_4 _standamplitudeymodifier_4 _crouchcycletimemodifier_4 _crouchamplitudexmodifier_4 _crouchamplitudeymodifier_4 _movecycletimemodifier_4 _moveamplitudexmodifier_4 _moveamplitudeymodifier_4) (break `AnimPlayerIdleSwayData` _value))
  (if (and (and (`KismetSystemLibrary.IsValid` Target) (>= Factor 0.0)) (<= Factor 4.0))
    (set `self.WorkingSway` (`AnimInstancePlayer.IdleSwayData` Target))
    (set `self.BaselineSway` (`self.WorkingSway`))
    (setmembers `AnimPlayerIdleSwayData` :`StructRef` (`self.BaselineSway`) :`StandAmplitudeXModifier` (`KismetMathLibrary.SelectFloat` _standamplitudexmodifier_3 _standamplitudexmodifier (and (and _returnvalue_2 _returnvalue) (`KismetMathLibrary.NearlyEqual_FloatFloat` _standamplitudexmodifier _standamplitudexmodifier_4))) :`StandAmplitudeYModifier` (`KismetMathLibrary.SelectFloat` _standamplitudeymodifier_3 _standamplitudeymodifier (and (and _returnvalue_2 _returnvalue) (`KismetMathLibrary.NearlyEqual_FloatFloat` _standamplitudeymodifier _standamplitudeymodifier_4))) :`CrouchAmplitudeXModifier` (`KismetMathLibrary.SelectFloat` _crouchamplitudexmodifier_3 _crouchamplitudexmodifier (and (and _returnvalue_2 _returnvalue) (`KismetMathLibrary.NearlyEqual_FloatFloat` _crouchamplitudexmodifier _crouchamplitudexmodifier_4))) :`CrouchAmplitudeYModifier` (`KismetMathLibrary.SelectFloat` _crouchamplitudeymodifier_3 _crouchamplitudeymodifier (and (and _returnvalue_2 _returnvalue) (`KismetMathLibrary.NearlyEqual_FloatFloat` _crouchamplitudeymodifier _crouchamplitudeymodifier_4))) :`MoveAmplitudeXModifier` (`KismetMathLibrary.SelectFloat` _moveamplitudexmodifier_3 _moveamplitudexmodifier (and (and _returnvalue_2 _returnvalue) (`KismetMathLibrary.NearlyEqual_FloatFloat` _moveamplitudexmodifier _moveamplitudexmodifier_4))) :`MoveAmplitudeYModifier` (`KismetMathLibrary.SelectFloat` _moveamplitudeymodifier_3 _moveamplitudeymodifier (and (and _returnvalue_2 _returnvalue) (`KismetMathLibrary.NearlyEqual_FloatFloat` _moveamplitudeymodifier _moveamplitudeymodifier_4))))
    (`BlueprintMapLibrary.Map_Add` (`self.OriginalSway`) Target (`self.BaselineSway`))
    (setmembers `AnimPlayerIdleSwayData` :`StructRef` (`self.WorkingSway`) :`StandAmplitudeXModifier` (- (* (+ _standamplitudexmodifier_2 1.0) Factor) 1.0) :`StandAmplitudeYModifier` (- (* (+ _standamplitudeymodifier_2 1.0) Factor) 1.0) :`CrouchAmplitudeXModifier` (- (* (+ _crouchamplitudexmodifier_2 1.0) Factor) 1.0) :`CrouchAmplitudeYModifier` (- (* (+ _crouchamplitudeymodifier_2 1.0) Factor) 1.0) :`MoveAmplitudeXModifier` (- (* (+ _moveamplitudexmodifier_2 1.0) Factor) 1.0) :`MoveAmplitudeYModifier` (- (* (+ _moveamplitudeymodifier_2 1.0) Factor) 1.0))
    (set `AnimInstancePlayer.IdleSwayData` (`self.WorkingSway`) Target)
    (`BlueprintMapLibrary.Map_Add` (`self.LastSway`) Target (`self.WorkingSway`))
    (`KismetArrayLibrary.Array_AddUnique` (`self.TrackedInstances`) Target)))

(event `ReleaseSway`
  (bind (_basecurve _staminaamplitudecurve _staminacycletimecurve _initialdelay _standcycletimemodifier _standamplitudexmodifier _standamplitudeymodifier _crouchcycletimemodifier _crouchamplitudexmodifier _crouchamplitudeymodifier _movecycletimemodifier _moveamplitudexmodifier _moveamplitudeymodifier) (break `AnimPlayerIdleSwayData` (`self.WorkingSway`)))
  (for _array_element (`self.TrackedInstances`)
    (if (`KismetSystemLibrary.IsValid` _array_element)
      (set `self.WorkingSway` (`AnimInstancePlayer.IdleSwayData` _array_element))
      (bind (_value _returnvalue) (`BlueprintMapLibrary.Map_Find` (`self.OriginalSway`) _array_element))
      (bind (_basecurve_2 _staminaamplitudecurve_2 _staminacycletimecurve_2 _initialdelay_2 _standcycletimemodifier_2 _standamplitudexmodifier_2 _standamplitudeymodifier_2 _crouchcycletimemodifier_2 _crouchamplitudexmodifier_2 _crouchamplitudeymodifier_2 _movecycletimemodifier_2 _moveamplitudexmodifier_2 _moveamplitudeymodifier_2) (break `AnimPlayerIdleSwayData` _value))
      (bind (_value_2 _returnvalue_2) (`BlueprintMapLibrary.Map_Find` (`self.LastSway`) _array_element))
      (bind (_basecurve_3 _staminaamplitudecurve_3 _staminacycletimecurve_3 _initialdelay_3 _standcycletimemodifier_3 _standamplitudexmodifier_3 _standamplitudeymodifier_3 _crouchcycletimemodifier_3 _crouchamplitudexmodifier_3 _crouchamplitudeymodifier_3 _movecycletimemodifier_3 _moveamplitudexmodifier_3 _moveamplitudeymodifier_3) (break `AnimPlayerIdleSwayData` _value_2))
      (setmembers `AnimPlayerIdleSwayData` :`StructRef` (`self.WorkingSway`) :`StandAmplitudeXModifier` (`KismetMathLibrary.SelectFloat` _standamplitudexmodifier_2 _standamplitudexmodifier (and (and _returnvalue _returnvalue_2) (`KismetMathLibrary.NearlyEqual_FloatFloat` _standamplitudexmodifier _standamplitudexmodifier_3))) :`StandAmplitudeYModifier` (`KismetMathLibrary.SelectFloat` _standamplitudeymodifier_2 _standamplitudeymodifier (and (and _returnvalue _returnvalue_2) (`KismetMathLibrary.NearlyEqual_FloatFloat` _standamplitudeymodifier _standamplitudeymodifier_3))) :`CrouchAmplitudeXModifier` (`KismetMathLibrary.SelectFloat` _crouchamplitudexmodifier_2 _crouchamplitudexmodifier (and (and _returnvalue _returnvalue_2) (`KismetMathLibrary.NearlyEqual_FloatFloat` _crouchamplitudexmodifier _crouchamplitudexmodifier_3))) :`CrouchAmplitudeYModifier` (`KismetMathLibrary.SelectFloat` _crouchamplitudeymodifier_2 _crouchamplitudeymodifier (and (and _returnvalue _returnvalue_2) (`KismetMathLibrary.NearlyEqual_FloatFloat` _crouchamplitudeymodifier _crouchamplitudeymodifier_3))) :`MoveAmplitudeXModifier` (`KismetMathLibrary.SelectFloat` _moveamplitudexmodifier_2 _moveamplitudexmodifier (and (and _returnvalue _returnvalue_2) (`KismetMathLibrary.NearlyEqual_FloatFloat` _moveamplitudexmodifier _moveamplitudexmodifier_3))) :`MoveAmplitudeYModifier` (`KismetMathLibrary.SelectFloat` _moveamplitudeymodifier_2 _moveamplitudeymodifier (and (and _returnvalue _returnvalue_2) (`KismetMathLibrary.NearlyEqual_FloatFloat` _moveamplitudeymodifier _moveamplitudeymodifier_3))))
      (set `AnimInstancePlayer.IdleSwayData` (`self.WorkingSway`) _array_element)))
  (`BlueprintMapLibrary.Map_Clear` (`self.OriginalSway`))
  (`BlueprintMapLibrary.Map_Clear` (`self.LastSway`))
  (`KismetArrayLibrary.Array_Clear` (`self.TrackedInstances`)))

(event `self.OnWorldBeginPlay`
  (params (World :type "World Object Reference"))
  (bind (_value _returnvalue) (`BlueprintMapLibrary.Map_Find` (`self.ProfileValues`) "menu.enabled"))
  (bind (_value_2 _returnvalue_2) (`BlueprintMapLibrary.Map_Find` (`self.ProfileValues`) "visual.sway"))
  (bind _returnvalue_3 (and (and (and (`self.ProfileReady`) _returnvalue_2) (>= _value_2 1.0)) (<= _value_2 5.0)))
  (set `self.MenuEnabled` (and (and (`self.ProfileReady`) _returnvalue) (== _value 1.0)))
  (if (or _returnvalue_3 (`self.MenuEnabled`))
    (set `self.SwayFactor` (`KismetMathLibrary.SelectFloat` (- _value_2 1.0) 1.0 _returnvalue_3))
    (set `self.ProfileSwayFactor` (`self.SwayFactor`))
    (set `self.VisualEnabled` true)
    (`self.SetTickEnabled` self true)))

(event `self.OnTick`
  (params (DeltaTime :type "Float (single-precision)"))
  (bind _returnvalue (`GameplayStatics.GetPlayerController` 0))
  (bind _swayfactor (`/S2TRuntimeLab/Menu/WBP_S2TMenu.SwayFactor` (`self.LiveMenu`)))
  (set `self.SwayFactor` (`self.ProfileSwayFactor`))
  (if (`self.MenuEnabled`)
    (if (`KismetSystemLibrary.IsValid` (`self.LiveMenu`))
      (if (`KismetSystemLibrary.IsValid` _returnvalue) :!label _label_3
        (if (and (and (and (and (and (and (`Controller.IsLocalController` _returnvalue) (== (`UserWidget.GetOwningPlayer` (`self.LiveMenu`)) _returnvalue)) (`/S2TRuntimeLab/Menu/WBP_S2TMenu.ProfileReady` (`self.LiveMenu`))) (`KismetStringLibrary.EqualEqual_StrStr` (`/S2TRuntimeLab/Menu/WBP_S2TMenu.SourceProfile` (`self.LiveMenu`)) (`/S2TRuntimeLab/BP_S2TProfile.ProfileData` (`self.LoadedProfile`)))) (`Widget.IsInViewport` (`self.LiveMenu`))) (>= _swayfactor 0.0)) (<= _swayfactor 4.0))
          (set `self.SwayFactor` _swayfactor)
          (else
            (set `self.LiveMenu` null :!label _label_4)))
        (else
          (goto _label_4)))
      (else
        (set `self.MenuSearchElapsed` (+ (`self.MenuSearchElapsed`) DeltaTime))
        (if (>= (`self.MenuSearchElapsed`) 0.5)
          (set `self.MenuSearchElapsed` 0.0)
          (bind _foundwidgets (`WidgetBlueprintLibrary.GetAllWidgetsOfClass` "/S2TRuntimeLab/Menu/WBP_S2TMenu.WBP_S2TMenu_C"))
          (if (== (`KismetArrayLibrary.Array_Length` _foundwidgets) 1)
            (bind _aswbp_s2tmenu (cast `/S2TRuntimeLab/Menu/WBP_S2TMenu` (`KismetArrayLibrary.Array_Get` _foundwidgets))
              (:`then`
                (set `self.LiveMenu` _aswbp_s2tmenu)
                (goto _label_3))
              (:`CastFailed`
                _)))))))
  (if (`self.VisualEnabled`)
    (if (!= (`self.SwayFactor`) 1.0)
      (bind _aspc (cast `PC` (`GameplayStatics.GetPlayerPawn` 0))
        (:`then`
          (if (`PC.IsInCinematic` _aspc)
            (`self.ReleaseSway` :!label _label_5)
            (else
              (for _array_element (`Actor.K2_GetComponentsByClass` _aspc "/Script/Engine.SkeletalMeshComponent")
                (bind _asskeletal_mesh_component (cast `SkeletalMeshComponent` _array_element))
                (bind _asanim_instance_player (cast `AnimInstancePlayer` (`SkeletalMeshComponent.GetAnimInstance` _asskeletal_mesh_component)))
                (`self.ApplySway` _asanim_instance_player (`self.SwayFactor`))))))
        (:`CastFailed`
          (goto _label_5)))
      (else
        (goto _label_5)))
    (else
      (goto _label_5))))

(event `self.PreDeinitialize`
  (`self.SetTickEnabled` self false)
  (set `self.LiveMenu` null)
  (`self.ReleaseSway`))

(event `ParseLoadedProfile`
  (goto _label))