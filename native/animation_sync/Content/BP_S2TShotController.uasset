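; Ticking controller that dampens the player's weapon shot animation by a saved profile setting.
; Loads and strictly validates a key=value save profile, turning `visual.shot` into a blend factor.
; Links ABP_S2TShotMix into the player's weapon layer, with montage evaluation on for its Normal branch and off for Baseline.
; Applies that weight while firing, restores full weight otherwise, and unlinks during cinematics or when validation fails.
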(event `self.OnInitialized`
  (bind _loadedprofile (`self.LoadedProfile`))
  (bind _profilelines (`self.ProfileLines`))
  (bind _returnvalue (`KismetArrayLibrary.Array_Length` _profilelines))
  (bind _profiledata (`/S2TRuntimeLab/BP_S2TProfile.ProfileData` _loadedprofile))
  (bind _returnvalue_2 (`KismetStringLibrary.Len` _profiledata))
  (set `self.LoadedProfile` null)
  (bind _returnvalue_3 (`GameplayStatics.LoadGameFromSlot` (`self.ProfileSlot`)))
  (bind _asbp_s2tprofile (cast `/S2TRuntimeLab/BP_S2TProfile` _returnvalue_3)
    (:`then`
      (set `self.LoadedProfile` _asbp_s2tprofile))
    (:`CastFailed`
      _))
  (set `self.ProfileReady` false :!label _label)
  (`BlueprintMapLibrary.Map_Clear` (`self.ProfileValues`))
  (if (`KismetSystemLibrary.IsValid` _loadedprofile)
    (if (and (and (== (`/S2TRuntimeLab/BP_S2TProfile.ProfileSchema` _loadedprofile) 1) (>= _returnvalue_2 4)) (<= _returnvalue_2 64000))
      (set `self.ProfileLines` (`KismetStringLibrary.ParseIntoArray` _profiledata "\n" false))
      (if (and (>= _returnvalue 1) (<= _returnvalue 2048))
        (set `self.ProfileReady` true)
        (for (_array_element _array_index) _profilelines
          (if (== _array_index 0)
            (if (not (`KismetStringLibrary.EqualEqual_StrStr` _array_element "S2T1"))
              (set `self.ProfileReady` false :!label _label_2))
            (else
              (bind (_lefts _rights _returnvalue_4) (`KismetStringLibrary.Split` _array_element "="))
              (if _returnvalue_4
                (bind _returnvalue_5 (`KismetStringLibrary.Conv_StringToDouble` _rights))
                (if (and (and (and (and (`KismetStringLibrary.IsNumeric` _rights) (> _returnvalue_5 0.0)) (<= _returnvalue_5 100.0)) (> (`KismetStringLibrary.Len` _lefts) 0)) (not (`BlueprintMapLibrary.Map_Contains` (`self.ProfileValues`) _lefts)))
                  (`BlueprintMapLibrary.Map_Add` (`self.ProfileValues`) _lefts _returnvalue_5)
                  (else
                    (goto _label_2)))
                (else
                  (goto _label_2))))))
        (if (not (`self.ProfileReady`))
          (`BlueprintMapLibrary.Map_Clear` (`self.ProfileValues`)))))))

(event `ReleaseShotLayer`
  (if (`KismetSystemLibrary.IsValid` (`self.OwnedOuter`))
    (if (and (`KismetSystemLibrary.IsValid` (`self.OwnedMix`)) (== (`AnimInstance.GetLinkedAnimLayerInstanceByClass` (`self.OwnedOuter`) "/S2TRuntimeLab/Firing/ABP_S2TShotMix.ABP_S2TShotMix_C" false) (`self.OwnedMix`)))
      (set `/S2TRuntimeLab/Firing/ABP_S2TShotMix.ShotWeight` 1.0 (`self.OwnedMix`))
      (`AnimInstance.UnlinkAnimClassLayers` (`self.OwnedOuter`) "/S2TRuntimeLab/Firing/ABP_S2TShotMix.ABP_S2TShotMix_C")))
  (set `self.OwnedMix` null)
  (set `self.OwnedOuter` null))

(event `self.OnWorldBeginPlay`
  (params (World :type "World Object Reference"))
  (bind (_value _returnvalue) (`BlueprintMapLibrary.Map_Find` (`self.ProfileValues`) "visual.shot"))
  (if (and (and (and (`self.ProfileReady`) _returnvalue) (>= _value 1.0)) (< _value 2.0))
    (set `self.ShotFactor` (- _value 1.0))
    (set `self.ShotEnabled` true)
    (`self.SetTickEnabled` self true)))

(event `self.OnTick`
  (params (DeltaTime :type "Float (single-precision)"))
  (bind _returnvalue (`AnimInstance.GetLinkedAnimLayerInstanceByGroup` (`self.WorkingOuter`) "BaseAnimLayer"))
  (bind _returnvalue_2 (`AnimInstance.GetLinkedAnimGraphInstanceByTag` (`self.OwnedMix`) "S2TBaseline"))
  (bind _returnvalue_3 (`AnimInstance.GetLinkedAnimGraphInstanceByTag` (`self.OwnedMix`) "S2TNormal"))
  (bind _returnvalue_4 (`AnimInstance.GetLinkedAnimLayerInstanceByClass` _returnvalue_2 "/Game/_STALKER2/Animations/Player/AnimLayers/AnimBP_PlayerWeaponLayer.AnimBP_PlayerWeaponLayer_C" false))
  (bind _returnvalue_5 (`AnimInstance.GetLinkedAnimLayerInstanceByClass` _returnvalue_3 "/Game/_STALKER2/Animations/Player/AnimLayers/AnimBP_PlayerWeaponLayer.AnimBP_PlayerWeaponLayer_C" false))
  (if (`self.ShotEnabled`)
    (bind _aspc (cast `PC` (`GameplayStatics.GetPlayerPawn` 0))
      (:`then`
        (if (not (`PC.IsInCinematic` _aspc))
          (bind _returnvalue_6 (`SkeletalMeshComponent.GetAnimInstance` (`Character.Mesh` _aspc)))
          (if (`KismetSystemLibrary.IsValid` _returnvalue_6)
            (set `self.WorkingOuter` (`AnimInstance.GetLinkedAnimLayerInstanceByClass` _returnvalue_6 "/Game/_STALKER2/Animations/Player/AnimLayers/AnimBP_PlayerWeaponLayer.AnimBP_PlayerWeaponLayer_C" false))
            (if (`KismetSystemLibrary.IsValid` (`self.WorkingOuter`))
              (if (== (`self.WorkingOuter`) (`self.OwnedOuter`))
                (if (and (`KismetSystemLibrary.IsValid` (`self.OwnedMix`)) (== (`AnimInstance.GetLinkedAnimLayerInstanceByClass` (`self.OwnedOuter`) "/S2TRuntimeLab/Firing/ABP_S2TShotMix.ABP_S2TShotMix_C" false) (`self.OwnedMix`))) :!label _label_3
                  (bind _returnvalue_7 (`PC.GetWeaponInHandsMeshComponent` _aspc))
                  (if (`KismetSystemLibrary.IsValid` _returnvalue_7)
                    (bind _returnvalue_8 (`SkeletalMeshComponent.GetAnimInstance` _returnvalue_7))
                    (if (`KismetSystemLibrary.IsValid` _returnvalue_8)
                      (bind _returnvalue_9 (`AnimInstance.GetCurrentActiveMontage` _returnvalue_8))
                      (if (or (and (`KismetSystemLibrary.IsValid` _returnvalue_9) (`KismetStringLibrary.Contains` (`KismetSystemLibrary.GetObjectName` _returnvalue_9) "_shoot")) (and (not (`KismetSystemLibrary.IsValid` _returnvalue_9)) (`PC.IsFiring` _aspc)))
                        (set `/S2TRuntimeLab/Firing/ABP_S2TShotMix.ShotWeight` (`self.ShotFactor`) (`self.OwnedMix`))
                        (else
                          (set `/S2TRuntimeLab/Firing/ABP_S2TShotMix.ShotWeight` 1.0 (`self.OwnedMix`) :!label _label_4)))
                      (else
                        (goto _label_4)))
                    (else
                      (goto _label_4)))
                  (else
                    (`self.ReleaseShotLayer` :!label _label_5)))
                (else
                  (`self.ReleaseShotLayer`)
                  (if (or (not (`KismetSystemLibrary.IsValid` _returnvalue)) (== _returnvalue (`self.WorkingOuter`)))
                    (`AnimInstance.LinkAnimClassLayers` (`self.WorkingOuter`) "/S2TRuntimeLab/Firing/ABP_S2TShotMix.ABP_S2TShotMix_C")
                    (set `self.OwnedOuter` (`self.WorkingOuter`))
                    (bind _asabp_s2tshot_mix (cast `/S2TRuntimeLab/Firing/ABP_S2TShotMix` (`AnimInstance.GetLinkedAnimLayerInstanceByClass` (`self.OwnedOuter`) "/S2TRuntimeLab/Firing/ABP_S2TShotMix.ABP_S2TShotMix_C" false))
                      (:`then`
                        (set `self.OwnedMix` _asabp_s2tshot_mix)
                        (if (`KismetSystemLibrary.IsValid` _returnvalue_3)
                          (if (`KismetSystemLibrary.IsValid` _returnvalue_5)
                            (`AnimInstance.SetUseMainInstanceMontageEvaluationData` _returnvalue_5 true)
                            (if (`KismetSystemLibrary.IsValid` _returnvalue_2)
                              (if (`KismetSystemLibrary.IsValid` _returnvalue_4)
                                (`AnimInstance.SetUseMainInstanceMontageEvaluationData` _returnvalue_4 false)
                                (goto _label_3)
                                (else
                                  (goto _label_5)))
                              (else
                                (goto _label_5)))
                            (else
                              (goto _label_5)))
                          (else
                            (goto _label_5))))
                      (:`CastFailed`
                        (goto _label_5))))))
              (else
                (goto _label_5)))
            (else
              (goto _label_5)))
          (else
            (goto _label_5))))
      (:`CastFailed`
        (goto _label_5)))
    (else
      (goto _label_5))))

(event `ParseLoadedProfile`
  (goto _label))